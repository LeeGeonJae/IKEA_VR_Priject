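; Selectable living-room table furniture actor for a VR scene, with a material setter for slot 0.
; Selecting it triggers CBComponent's click color and copies its mesh to every SelectFurnitureActor; releasing restores color through CBComponent.
; Selection also clears existing widget actors, then spawns an info widget (name, size, description) and SelectActor_Widget_11 at the right motion controller.
; The SelectActorWidget variant, which passes mesh and scale, is not called here.
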(event EventBeginPlay)

(event Collision|EventActorBeginOverlap
  (params (OtherActor :type Actor%20Object%20Reference)))

(event EventTick
  (params (DeltaSeconds :type Float%20%28single-precision%29)))

(event EventOnSelect
  (Default|ClickColor (Variables|Default|GetCB_Component))
  (CallFunction|SetSceneActorMesh)
  (CallFunction|SelectActorWidget2)
  (CallFunction|SelectActorWidget11))

(event EventOnEndOverlap)

(event EventOnBeginOverlap)

(event EventOnRelease
  (Default|ReleaseColor (Variables|Default|GetCB_Component)))

(fn ConstructionScript)

(fn SetSceneActorMesh
  (bind _outactors (Actor|GetAllActorsOfClass "/Game/Test/Project/Blueprint/Scene/SelectFurnitureActor.SelectFurnitureActor_C"))
  (for _array_element _outactors
    (Default|SetNewMesh _array_element (Variables|/Script/Engine.StaticMeshComponent|GetStaticMesh (Variables|Default|GetStaticMesh)))))

(fn SelectActorWidget
  (bind _outactors (Actor|GetAllActorsOfClass "/Game/Test/Project/Blueprint/SelectMoveActor/SelectActor_Widget.SelectActor_Widget_C"))
  (for _array_element _outactors
    (Actor|DestroyActor _array_element))
  (bind _asvrpawn (Utilities|Casting|CastToVRPawn (Game|Player|GetPlayerPawn 0)))
  (Game|SpawnActorfromClass "/Game/Test/Project/Blueprint/SelectMoveActor/SelectActor_Widget.SelectActor_Widget_C" (Transformation|GetWorldTransform (Variables|/Game/Test/Project/GameMode/VRPawn.VRPawn_C|GetMotionControllerRight _asvrpawn)) "Undefined" 0 self (Variables|/Script/Engine.StaticMeshComponent|GetStaticMesh (Variables|Default|GetStaticMesh)) (Transformation|GetWorldScale (Variables|Default|GetStaticMesh)) 0))

(fn SelectActorWidget2
  (bind _outactors (Actor|GetAllActorsOfClass "/Game/Test/Project/Blueprint/SelectMoveActor/SelectActor_Widget_2.SelectActor_Widget_2_C"))
  (for _array_element _outactors
    (Actor|DestroyActor _array_element))
  (bind _asvrpawn (Utilities|Casting|CastToVRPawn (Game|Player|GetPlayerPawn 0)))
  (Game|SpawnActorfromClass "/Game/Test/Project/Blueprint/SelectMoveActor/SelectActor_Widget_2.SelectActor_Widget_2_C" (Transformation|GetWorldTransform (Variables|/Game/Test/Project/GameMode/VRPawn.VRPawn_C|GetMotionControllerRight _asvrpawn)) "Undefined" 0 self (Variables|Default|GetStrName) (Variables|Default|GetStrSize) (Variables|Default|GetStrInformation) 0))

(fn SelectActorWidget11
  (bind _outactors (Actor|GetAllActorsOfClass "/Game/Test/Project/Blueprint/WidgetActor/AllWidgetActorDelete.AllWidgetActorDelete_C"))
  (for _array_element _outactors
    (Default|DeleteActor _array_element))
  (bind _asvrpawn (Utilities|Casting|CastToVRPawn (Game|Player|GetPlayerPawn 0)))
  (Game|SpawnActorfromClass "/Game/SDW/Blueprints/FurnitureColorWidget/SelectActor_Widget_11.SelectActor_Widget_11_C" (Transformation|GetWorldTransform (Variables|/Game/Test/Project/GameMode/VRPawn.VRPawn_C|GetMotionControllerRight _asvrpawn)) "Undefined" 0 self 0))

(fn SetMatirial
  (params (Material :type Material%20Interface%20Object%20Reference))
  (Rendering|Material|SetMaterial (Variables|Default|GetStaticMesh) 0 Material))