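; BP_Shower is an interactive shower that reacts to overlaps on its collider.
; Beginning overlap enables player input and, after a short delay, toggles visibility, adds a particle system component and toggles that component's visibility.
; Left click toggles the particle component again; ending overlap disables input and repeats the first visibility toggle.
; Each overlap adds a new particle component, and a ToggleActive helper function is not called here.
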(event OnComponentEndOverlap(Collider)
  (params (OverlappedComponent :type Primitive%20Component%20Object%20Reference) (OtherActor :type Actor%20Object%20Reference) (OtherComp :type Primitive%20Component%20Object%20Reference) (OtherBodyIndex :type Integer))
  (Input|DisableInput (Game|GetPlayerController 0))
  (Utilities|FlowControl|Delay 0.2)
  (Rendering|ToggleVisibility false))

(event OnComponentBeginOverlap(Collider)
  (params (OverlappedComponent :type Primitive%20Component%20Object%20Reference) (OtherActor :type Actor%20Object%20Reference) (OtherComp :type Primitive%20Component%20Object%20Reference) (OtherBodyIndex :type Integer) (bFromSweep :type Boolean) (SweepResult :type Hit%20Result%20Structure%20%28by%20ref%29))
  (Input|EnableInput (Game|GetPlayerController 0))
  (Utilities|FlowControl|Delay 0.2)
  (Rendering|ToggleVisibility false)
  (bind _returnvalue (AddComponent|AddParticleSystemComponent false))
  (Rendering|ToggleVisibility _returnvalue false))

(event Input|MouseEvents|LeftMouseButton
  (params (Key :type Key%20Structure :default "None"))
  (:Pressed
    (Rendering|ToggleVisibility (stale OnComponentBeginOverlap(Collider) _returnvalue) false)))

(fn ConstructionScript)

(fn NewFunction0
  (params (self2 :type Actor%20Component%20Object%20Reference))
  (Components|Activation|ToggleActive self2))