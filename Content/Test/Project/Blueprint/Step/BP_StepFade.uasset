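; BP_StepFade is a step Blueprint that runs a camera fade on the first player's view.
; StartStep calls the parent, starts a held fade from a high alpha, and sets a timer to call EndStep, which this file does not define.
; The timer fires before the fade finishes, so the step can end mid-fade.
; StopStep calls the parent and clears that timer, leaving the fade untouched.
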(event EventBeginPlay
  (|CallParentFunction) ; 지금 이 노드는 비활성 상태입니다. \n핀을 끌어서 다른 노드를 연결하면 활성화됩니다.
)

(event EventTick
  (params (DeltaSeconds :type Float%20%28single-precision%29)))

(fn ConstructionScript
  (|CallParentFunction))

(fn StartStep
  (|CallParentFunction)
  (CameraFades|StartCameraFade :self (Game|GetPlayerCameraManager 0) :FromAlpha 2.0 :Duration 2.0 :bHoldWhenFinished true)
  (Utilities|Time|SetTimerbyFunctionName 0 "EndStep" 1.0))

(fn StopStep
  (|CallParentFunction)
  (Utilities|Time|ClearTimerbyFunctionName 0 "EndStep"))