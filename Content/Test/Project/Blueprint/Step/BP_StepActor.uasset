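; BP_StepActor is a base actor that reacts to a game step sequence held by MH_GameState.
; On BeginPlay it binds to the game state's step-change event, calling StartStep when the new step matches MyStep and StopStep otherwise.
; StartStep and StopStep are empty hooks, while EndStep requests NextStep from the game state only if it equals the enum's NewEnumerator0.
; The construction script shows Comment on a text render.
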(event EventBeginPlay
  (CallFunction|InitBind))

(fn ConstructionScript
  (Rendering|Components|TextRender|SetText (Variables|Default|GetTextRender) (Variables|Default|GetComment)))

(fn InitBind
  (bind _asmh_game_state (Utilities|Casting|CastToMH_GameState (Game|GetGameState)))
  (EventDispatchers|BindEventtoChangeStepEvent _asmh_game_state (EventDispatchers|CreateEvent :!event ChangeStepEvent)))

(fn ChangeStepEvent
  (params (ChangeStep :type EN_Step%20Enum :default "NewEnumerator0"))
  (if (Utilities|Enum|Equal(Enum) ChangeStep (Variables|Default|GetMyStep))
    (CallFunction|StartStep)
    (else
      (CallFunction|StopStep))))

(fn StartStep)

(fn EndStep
  (if (Utilities|Enum|Equal(Enum) (Variables|Default|GetNextStep) "NewEnumerator0")
    (bind _asmh_game_state (Utilities|Casting|CastToMH_GameState (Game|GetGameState)))
    (Default|ChangeStep _asmh_game_state (Variables|Default|GetNextStep))))

(fn StopStep)