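; BP_SelectArea is a step actor that completes when its area is selected.
; Starting the step enables collision on a Box, which is hidden at play start, and ending or stopping it disables that collision.
; Overlap begin and end events show and hide a Decal as a highlight, and OnSelect calls EndStep.
; StartStep, EndStep and StopStep all extend their parent versions.
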(event EventBeginPlay
  (|CallParentFunction)
  (Rendering|SetVisibility (Variables|Default|GetBox) false false))

(event Collision|EventActorBeginOverlap
  (params (OtherActor :type Actor%20Object%20Reference)))

(event EventTick
  (params (DeltaSeconds :type Float%20%28single-precision%29)))

(event EventOnBeginOverlap
  (Rendering|SetVisibility (Variables|Default|GetDecal) true false))

(event EventOnEndOverlap
  (Rendering|SetVisibility (Variables|Default|GetDecal) false false))

(event EventOnSelect
  (CallFunction|EndStep))

(fn ConstructionScript)

(fn StartStep
  (|CallParentFunction)
  (Collision|SetCollisionEnabled (Variables|Default|GetBox) "QueryAndPhysics"))

(fn EndStep
  (|CallParentFunction)
  (Collision|SetCollisionEnabled (Variables|Default|GetBox) "NoCollision"))

(fn StopStep
  (|CallParentFunction)
  (Collision|SetCollisionEnabled (Variables|Default|GetBox) "NoCollision"))