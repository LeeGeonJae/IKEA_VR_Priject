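; BP_StepTeleport is a step Blueprint that moves the player pawn to a PlayerStart.
; StartStep begins a one-second camera fade to full opacity and sets a timer of equal length for DoTeleport.
; DoTeleport applies the PlayerStart's location and rotation to the pawn, then calls EndStep, with no fade back in here.
; StopStep clears the pending timer.
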(event EventBeginPlay
  (|CallParentFunction) ; 지금 이 노드는 비활성 상태입니다. \n핀을 끌어서 다른 노드를 연결하면 활성화됩니다.
)

(event Collision|EventActorBeginOverlap
  (params (OtherActor :type Actor%20Object%20Reference)))

(event EventTick
  (params (DeltaSeconds :type Float%20%28single-precision%29)))

(fn ConstructionScript
  (|CallParentFunction))

(fn DoTeleport
  (bind _playerstart (Variables|Default|GetPlayerStart))
  (Transformation|SetActorLocationAndRotation (Game|Player|GetPlayerPawn 0) (Transformation|GetActorLocation _playerstart) (Transformation|GetActorRotation _playerstart))
  (CallFunction|EndStep))

(fn StartStep
  (|CallParentFunction)
  (CameraFades|StartCameraFade :self (Game|GetPlayerCameraManager 0) :ToAlpha 1.0 :Duration 1.0)
  (Utilities|Time|SetTimerbyFunctionName 0 "DoTeleport" 1.0))

(fn StopStep
  (|CallParentFunction)
  (Utilities|Time|ClearTimerbyFunctionName 0 "DoTeleport"))