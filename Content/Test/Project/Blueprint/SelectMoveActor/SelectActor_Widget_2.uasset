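; VR info popup actor that shows a selected actor's name, size and information on a world-space widget.
; On BeginPlay it line-traces along the VRPawn's right-hand widget interaction ray and, if it hits SelectActor, places the widget above the impact point and fills its SelectActor_SceneWidget text; otherwise it destroys itself.
; While SelectActor is valid, Tick rotates the widget to face the player camera.
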(event EventBeginPlay
  ;[1 1 1] 액터 생산 초기 세팅
  (bind _asvrpawn (Utilities|Casting|CastToVRPawn (Game|Player|GetPlayerPawn 0)))
  (Variables|Default|SetWidget%20Interaction%20Right (Variables|/Game/Test/Project/GameMode/VRPawn.VRPawn_C|GetWidgetInteractionRight _asvrpawn))
  (bind _outhit (Collision|LineTraceForObjects (Transformation|GetWorldLocation (Variables|/Game/Test/Project/GameMode/VRPawn.VRPawn_C|GetWidgetInteractionRight _asvrpawn)) (+ (Transformation|GetWorldLocation (Variables|/Game/Test/Project/GameMode/VRPawn.VRPawn_C|GetWidgetInteractionRight _asvrpawn)) (* (Math|Vector|GetForwardVector (Variables|/Game/Test/Project/GameMode/VRPawn.VRPawn_C|GetWidgetInteractionRight _asvrpawn)) (Variables|/Script/UMG.WidgetInteractionComponent|GetInteractionDistance (Variables|/Game/Test/Project/GameMode/VRPawn.VRPawn_C|GetWidgetInteractionRight _asvrpawn)))) (Utilities|Array|MakeArray "ObjectTypeQuery2" "ObjectTypeQuery1" "ObjectTypeQuery3" "ObjectTypeQuery4" "ObjectTypeQuery5") false 0 "None"))
  (if (== (.HitActor (Collision|BreakHitResult _outhit)) (Variables|Default|GetSelectActor))
    (Transformation|SetWorldLocation (Variables|Default|GetWidget) (Math|Vector|MakeVector (- (.X (Math|Vector|BreakVector (.ImpactPoint (Collision|BreakHitResult _outhit)))) 0.0) (+ (.Y (Math|Vector|BreakVector (.ImpactPoint (Collision|BreakHitResult _outhit)))) 0.0) (+ (.Z (Math|Vector|BreakVector (.ImpactPoint (Collision|BreakHitResult _outhit)))) 125.0)) false false)
    (CallFunction|SetText (Variables|Default|GetStrName) (Variables|Default|GetStrSize) (Variables|Default|GetStrInformation))
    (else
      (CallFunction|Destory))))

(event EventTick
  (params (DeltaSeconds :type Float%20%28single-precision%29))
  ;[1 1 1] Widget 생성 위치, 플레이어를 향해 바라보기
  (Utilities|IsValid (Variables|Default|GetSelectActor)
    (:Is%20Valid
      (Transformation|SetWorldRotation (Variables|Default|GetWidget) (Math|Rotator|FindLookatRotation (Transformation|GetWorldLocation (Variables|Default|GetWidget)) (Transformation|GetActorLocation (Game|GetPlayerCameraManager 0))) false false))))

(fn ConstructionScript)

(fn Destory
  (Actor|DestroyActor))

(fn SetText
  (params (Name :type Text) (Size :type Text) (Information :type Text))
  (bind _asselect_actor_scene_widget (Utilities|Casting|CastToSelectActor_SceneWidget (UserInterface|GetWidget (Variables|Default|GetWidget))))
  (Default|SetText _asselect_actor_scene_widget Name Size Information))