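; InteriorZoneActor is a VR-selectable interior object that shows a configurable mesh, applied to its static mesh component on BeginPlay.
; On select, it destroys every existing SelectActor_Widget and spawns a new one at the VRPawn's right motion controller, passing itself, its mesh and world scale.
; A helper sets the mesh's material, while the overlap and release events are empty.
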(event EventBeginPlay
  (Components|StaticMesh|SetStaticMesh (Variables|Default|GetStaticMesh) (Variables|Default|GetSelectMesh)))

(event Collision|EventActorBeginOverlap
  (params (OtherActor :type Actor%20Object%20Reference)))

(event EventTick
  (params (DeltaSeconds :type Float%20%28single-precision%29)))

(event EventOnSelect
  (CallFunction|SelectActorWidget))

(event EventOnEndOverlap)

(event EventOnBeginOverlap)

(event EventOnRelease)

(fn ConstructionScript)

(fn SelectActorWidget
  (bind _outactors (Actor|GetAllActorsOfClass "/Game/Test/Project/Blueprint/SelectMoveActor/SelectActor_Widget.SelectActor_Widget_C"))
  (for _array_element _outactors
    (Actor|DestroyActor _array_element))
  (bind _asvrpawn (Utilities|Casting|CastToVRPawn (Game|Player|GetPlayerPawn 0)))
  (Game|SpawnActorfromClass "/Game/Test/Project/Blueprint/SelectMoveActor/SelectActor_Widget.SelectActor_Widget_C" (Transformation|GetWorldTransform (Variables|/Game/Test/Project/GameMode/VRPawn.VRPawn_C|GetMotionControllerRight _asvrpawn)) "Undefined" 0 self (Variables|/Script/Engine.StaticMeshComponent|GetStaticMesh (Variables|Default|GetStaticMesh)) (Transformation|GetWorldScale (Variables|Default|GetStaticMesh)) 0))

(fn SetMatirial
  (params (Material :type Material%20Interface%20Object%20Reference))
  (Rendering|Material|SetMaterial (Variables|Default|GetStaticMesh) 0 Material))