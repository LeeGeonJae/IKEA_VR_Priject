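; BP_SelectMoveActor is a translucent placement preview for putting a selected mesh into the world in VR.
; On BeginPlay it applies the selected mesh with a frosted-glass material and takes the VR pawn's right WidgetInteraction as its aim.
; Tick line-traces along that aim against WorldStatic, moving the preview and Niagara laser endpoint to the hit or laser's end.
; Right stick X yaws the preview; right trigger spawns InteriorZoneActor at its transform and destroys it.
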(event EventBeginPlay
  (bind _staticmesh (Variables|Default|GetStaticMesh))
  ;[1 1 1] Widget Interaction right 변수 지정
  (bind _asvrpawn (Utilities|Casting|CastToVRPawn (Game|Player|GetPlayerPawn 0)))
  (Variables|Default|SetWidgetInteraction (Variables|/Game/Test/Project/GameMode/VRPawn.VRPawn_C|GetWidgetInteractionRight _asvrpawn))
  ;[1 1 1] 초기 세팅, Enable Input
  (Transformation|SetWorldRotation (Variables|Default|GetStaticMesh) "0, 0, 0" false false)
  (Input|EnableInput (Game|GetPlayerController 0))
  ;[1 1 1] 스태틱 메쉬 지정, 머티리얼 변경
  (Components|StaticMesh|SetStaticMesh (Variables|Default|GetStaticMesh) (Variables|Default|GetSelectActorMesh))
  (for _index (range 0 (- (Rendering|Material|GetNumMaterials _staticmesh) 1))
    (Rendering|Material|SetMaterial _staticmesh _index "/DatasmithContent/Materials/StdTranslucent/M_StdTranslucentFrostedGlass.M_StdTranslucentFrostedGlass")))

(event EventTick
  (params (DeltaSeconds :type Float%20%28single-precision%29))
  (bind _menulaser (Variables|Default|GetMenuLaser))
  (bind _lasercur (Variables|Default|GetLaserCur))
  (bind _menulaser_2 (Variables|Default|GetMenuLaser))
  (bind _widgetinteraction (Variables|Default|GetWidgetInteraction))
  (bind _widgetinteraction_2 (Variables|Default|GetWidgetInteraction))
  (bind _returnvalue (Transformation|GetWorldLocation _widgetinteraction_2))
  (bind _returnvalue_2 (Math|Vector|GetForwardVector _widgetinteraction_2))
  (bind _returnvalue_3 (Transformation|GetWorldLocation _widgetinteraction))
  (bind _returnvalue_4 (* _returnvalue_2 _lasercur))
  (bind _returnvalue_5 (+ _returnvalue _returnvalue_4))
  (bind (_outhit _returnvalue_6) (Collision|LineTraceForObjects _returnvalue_3 (+ _returnvalue_3 (* (Math|Vector|GetForwardVector _widgetinteraction) (Variables|Default|GetLaserCur))) (Utilities|Array|MakeArray "ObjectTypeQuery1") false 0 "None"))
  (if _returnvalue_6
    ;[1 1 1] 벽에 부딪혔을 때,
    (Class|NiagaraDataInterfaceArrayFunctionLibrary|SetNiagaraArrayVectorValue _menulaser_2 "User.PointArray" 0 (Transformation|GetWorldLocation (Variables|Default|GetWidgetInteraction)) false) ; MenuLaser start location
    (Class|NiagaraDataInterfaceArrayFunctionLibrary|SetNiagaraArrayVectorValue _menulaser_2 "User.PointArray" 1 (.ImpactPoint (Collision|BreakHitResult _outhit)) false) ; MenuLaser end location
    (Transformation|SetWorldLocation (Variables|Default|GetStaticMesh) (.ImpactPoint (Collision|BreakHitResult _outhit)) false false)
    (else
      ;[1 1 1] 레이저가 벽에 부딪히지 않았을 때
      (Class|NiagaraDataInterfaceArrayFunctionLibrary|SetNiagaraArrayVectorValue _menulaser "User.PointArray" 0 _returnvalue false) ; MenuLaser start location
      (Class|NiagaraDataInterfaceArrayFunctionLibrary|SetNiagaraArrayVectorValue _menulaser "User.PointArray" 1 _returnvalue_5 false) ; MenuLaser end location
      (Transformation|SetWorldLocation (Variables|Default|GetStaticMesh) _returnvalue_5 false false))))

(event Input|ActionEvents|InputActionTriggerRight
  (params (Key :type Key%20Structure))
  ;[1 1 1] 액터 이동 완료
  (:Pressed
    (Game|SpawnActorfromClass "/Game/Test/Project/Blueprint/SelectMoveActor/InteriorZone/InteriorZoneActor.InteriorZoneActor_C" (Transformation|GetWorldTransform (Variables|Default|GetStaticMesh)) "Undefined" 0 (Variables|Default|GetSelectActorMesh) 0)
    (Actor|DestroyActor)))

(event Input|AxisEvents|InputAxisMovementAxisRight_X
  (params (AxisValue :type Float%20%28single-precision%29))
  ;[1 1 1] 회전
  (Transformation|AddWorldRotation (Variables|Default|GetStaticMesh) (Math|Rotator|MakeRotator 0.0 0.0 AxisValue) false false))

(fn ConstructionScript)