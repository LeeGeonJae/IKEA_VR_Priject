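; Helper actor Blueprint that clears every SelectActor_Widget actor variant from the level.
; Its DeleteActor function runs a Sequence with one branch per widget class, thirteen in all, each using GetAllActorsOfClass and destroying every instance found.
; The event graph and construction script are empty, so nothing in this asset calls DeleteActor itself.
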(event EventBeginPlay)

(event Collision|EventActorBeginOverlap
  (params (OtherActor :type Actor%20Object%20Reference)))

(event EventTick
  (params (DeltaSeconds :type Float%20%28single-precision%29)))

(fn ConstructionScript)

(fn DeleteActor
  (Utilities|FlowControl|Sequence
    (:then_0
      (bind _outactors (Actor|GetAllActorsOfClass "/Game/SDW/Blueprints/FurnitureColorWidget/SelectActor_Widget_4.SelectActor_Widget_4_C"))
      (for _array_element _outactors
        (Actor|DestroyActor _array_element)))
    (:then_1
      (bind _outactors_2 (Actor|GetAllActorsOfClass "/Game/Test/Project/Blueprint/SelectMoveActor/SelectActor_Widget_3.SelectActor_Widget_3_C"))
      (for _array_element_2 _outactors_2
        (Actor|DestroyActor _array_element_2)))
    (:then_2
      (bind _outactors_3 (Actor|GetAllActorsOfClass "/Game/Test/Project/Blueprint/SelectMoveActor/SelectActor_Widget.SelectActor_Widget_C"))
      (for _array_element_3 _outactors_3
        (Actor|DestroyActor _array_element_3)))
    (:then_3
      (bind _outactors_4 (Actor|GetAllActorsOfClass "/Game/Test/Project/Blueprint/SelectMoveActor/SelectActor_Widget_2.SelectActor_Widget_2_C"))
      (for _array_element_4 _outactors_4
        (Actor|DestroyActor _array_element_4)))
    (:then_4
      (bind _outactors_5 (Actor|GetAllActorsOfClass "/Game/SDW/Blueprints/FurnitureColorWidget/SelectActor_Widget_5.SelectActor_Widget_5_C"))
      (for _array_element_5 _outactors_5
        (Actor|DestroyActor _array_element_5)))
    (:then_5
      (bind _outactors_6 (Actor|GetAllActorsOfClass "/Game/SDW/Blueprints/FurnitureColorWidget/SelectActor_Widget_6.SelectActor_Widget_6_C"))
      (for _array_element_6 _outactors_6
        (Actor|DestroyActor _array_element_6)))
    (:then_6
      (bind _outactors_7 (Actor|GetAllActorsOfClass "/Game/SDW/Blueprints/FurnitureColorWidget/SelectActor_Widget_7.SelectActor_Widget_7_C"))
      (for _array_element_7 _outactors_7
        (Actor|DestroyActor _array_element_7)))
    (:then_7
      (bind _outactors_8 (Actor|GetAllActorsOfClass "/Game/SDW/Blueprints/FurnitureColorWidget/SelectActor_Widget_8.SelectActor_Widget_8_C"))
      (for _array_element_8 _outactors_8
        (Actor|DestroyActor _array_element_8)))
    (:then_8
      (bind _outactors_9 (Actor|GetAllActorsOfClass "/Game/SDW/Blueprints/FurnitureColorWidget/SelectActor_Widget_9.SelectActor_Widget_9_C"))
      (for _array_element_9 _outactors_9
        (Actor|DestroyActor _array_element_9)))
    (:then_9
      (bind _outactors_10 (Actor|GetAllActorsOfClass "/Game/SDW/Blueprints/FurnitureColorWidget/SelectActor_Widget_10.SelectActor_Widget_10_C"))
      (for _array_element_10 _outactors_10
        (Actor|DestroyActor _array_element_10)))
    (:then_10
      (bind _outactors_11 (Actor|GetAllActorsOfClass "/Game/SDW/Blueprints/FurnitureColorWidget/SelectActor_Widget_11.SelectActor_Widget_11_C"))
      (for _array_element_11 _outactors_11
        (Actor|DestroyActor _array_element_11)))
    (:then_11
      (bind _outactors_12 (Actor|GetAllActorsOfClass "/Game/SDW/Blueprints/FurnitureColorWidget/SelectActor_Widget_12.SelectActor_Widget_12_C"))
      (for _array_element_12 _outactors_12
        (Actor|DestroyActor _array_element_12)))
    (:then_12
      (bind _outactors_13 (Actor|GetAllActorsOfClass "/Game/SDW/Blueprints/FurnitureColorWidget/SelectActor_Widget_13.SelectActor_Widget_13_C"))
      (for _array_element_13 _outactors_13
        (Actor|DestroyActor _array_element_13)))))